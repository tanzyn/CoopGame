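; BP_Character is a character Blueprint that handles HUD creation and the held weapon.
; On BeginPlay it creates crosshair and ammo widgets and adds both to the viewport.
; Spawn Weapon destroys any current weapon, spawns the given type owned by the character, stores it as CurrentWeapon and attaches it to the mesh's RightHandSocket.
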(event `self.ReceiveBeginPlay`
  (bind _returnvalue (`|CreateWidget` "/Game/UI/WBP_Crosshair.WBP_Crosshair_C"))
  (bind _returnvalue_2 (`|CreateWidget` "/Game/UI/WBP_Ammo.WBP_Ammo_C"))
  (`UserWidget.AddToViewport` _returnvalue_2 0)
  (`UserWidget.AddToViewport` _returnvalue 0))

(fn `Spawn Weapon`
  (params (`Weapon Type` :type "SWeapon Class Reference"))
  (bind _current_weapon (`self.Current Weapon`))
  (`/Engine/EditorBlueprintResources/StandardMacros.IsValid` _current_weapon
    (:`Is Valid`
      (`self.K2_DestroyActor` _current_weapon))
    (:`Is Not Valid`
      _))
  (bind _returnvalue (`|SpawnActorFromClass` `Weapon Type` (`KismetMathLibrary.MakeTransform` (0.0 0.0 0.0)) "Undefined" "OverrideRootScale" self null))
  (bind _output_get (set `self.Current Weapon` _returnvalue))
  (`self.K2_AttachToComponent` _output_get (`self.Mesh`) "RightHandSocket" "KeepRelative" "KeepRelative" "KeepRelative" true))

(fn `UserConstructionScript`)